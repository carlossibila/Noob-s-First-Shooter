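; Player weapon component that handles aiming, firing and reloading of the equipped gun, and creates the player HUD.
; Enhanced Input events play arm montages by weapon-name section, while BP_Weapon messages return updated weapon data for the HUD.
; Shots line-trace from the camera, sending hits to BPI_Enemy actors or applying damage to others.
; Reload montage notifies move the magazine mesh between hand and gun sockets.
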(event `self.ReceiveBeginPlay`
  (`|ExecutionSequence`
    (:`then_0`
      (bind _asbp_fps_character (cast `/Game/GameFPS/core/BP_FPS_Character` (`GameplayStatics.GetPlayerCharacter` 0)))
      (bind _output_get (set `self.BP FPS Character` _asbp_fps_character))
      (set `self.BPC Player Inventory` (`/Game/GameFPS/core/BP_FPS_Character.BPC_PlayerInventory` _output_get)))
    (:`then_1`
      (`EnhancedInputSubsystemInterface.AddMappingContext` (pcsubsystem `EnhancedInputLocalPlayerSubsystem` (`GameplayStatics.GetPlayerController` 0)) "/Game/GameFPS/Inputs/IMC_EquippedWeapon.IMC_EquippedWeapon" 0 (struct)))
    (:`then_2`
      (bind _returnvalue (`|CreateWidget` "/Game/GameFPS/Widgets/WBP_PlayerUI.WBP_PlayerUI_C" (`GameplayStatics.GetPlayerController` 0)))
      (bind _output_get_2 (set `self.WBP_PlayerUI` _returnvalue))
      (`UserWidget.AddToViewport` _output_get_2 0))))

(event `EnhancedInput|/Game/GameFPS/Inputs/IA_Aim`
  (params (ActionValue :type Boolean) (ElapsedSeconds :type "Float (double-precision)") (TriggeredSeconds :type "Float (double-precision)") (InputAction :type "InputAction Object Reference" :default "/Game/GameFPS/Inputs/IA_Aim.IA_Aim"))
  ;[1 1 1] aim
  (:`Triggered`
    (if (not (or (`self.IsReloading`) (`self.IsShooting`)))
      (set `self.IsAming` true)
      (`/Game/GameFPS/Widgets/WBP_PlayerUI.UpdateCrosshairVisibility` (`self.WBP_PlayerUI`))))
  (:`Completed`
    (set `self.IsAming` false)
    (`/Game/GameFPS/Widgets/WBP_PlayerUI.UpdateCrosshairVisibility` (`self.WBP_PlayerUI`))))

(event `EnhancedInput|/Game/GameFPS/Inputs/IA_Shot`
  (params (ActionValue :type Boolean) (ElapsedSeconds :type "Float (double-precision)") (TriggeredSeconds :type "Float (double-precision)") (InputAction :type "InputAction Object Reference" :default "/Game/GameFPS/Inputs/IA_Shot.IA_Shot"))
  (bind _bp_fps_character (`self.BP FPS Character`))
  (bind ((`Name_11_56F88F3E450DAD7C284EAA808B049652` _name) (`FireRate_28_EBD23A0143F465FF33DD9C88ADAB6026` _firerate)) (break `/Game/GameFPS/Structures/S_WeaponBase` (`self.EquippedWeapon`)))
  (bind _camera (`/Game/GameFPS/core/BP_FPS_Character.Camera` _bp_fps_character))
  (bind _returnvalue (`SceneComponent.K2_GetComponentLocation` _camera))
  ;[0.6487 1 0.6273] Shot Manage
  (:`Triggered`
    (if (`self.CanShoot`)
      (`self.BP_Weapon`
        (:`then`
          ;;[1 1 1] check reload
          (if (`.Reload_1_B2AA21184498AA6A33DC0C8541A488C5` (break `/Game/GameFPS/Structures/S_WeaponBase` (`self.EquippedWeapon`)))
            ;;[1 1 1] action for empty mag
            (`/Engine/EditorBlueprintResources/StandardMacros.DoOnce` false :!label _label
              (:`Completed`
                (`GameplayStatics.PlaySoundAtLocation` "/Engine/VREditor/Sounds/UI/Flashlight_Switch.Flashlight_Switch" (`SceneComponent.K2_GetComponentLocation` (`/Game/GameFPS/core/Weapons/BP_Weapon.SK_Gun` (`self.BP_Weapon`))) (struct) 1.0 1.0 0.0 null null null null)
                (`KismetSystemLibrary.PrintString` "RELOAD")
                (`KismetSystemLibrary.Delay` (`.FireRate_28_EBD23A0143F465FF33DD9C88ADAB6026` (break `/Game/GameFPS/Structures/S_WeaponBase` (`self.EquippedWeapon`))))
                (set `self.IsShooting` false)
                (goto _label :!via `Reset`)))
            (elif (not (`self.IsShooting`))
              (`|PlayMontage` (`/Game/GameFPS/core/BP_FPS_Character.CharacterArms` (`self.BP FPS Character`)) "/Game/GameFPS/art/assaultRifle/animations/Montage_FP_Shot.Montage_FP_Shot" (* _firerate 10.0) 0.0 _name :!label _label_2
                (:`then`
                  ;;[1 1 1] Shot
                  (set `self.IsShooting` true)
                  (bind _updatedweaponstats (message `/Game/GameFPS/Interfaces/BPI_Weapon.Shot` (`self.BP_Weapon`) (`self.EquippedWeapon`)))
                  (bind _output_get (set `self.EquippedWeapon` _updatedweaponstats))
                  ;;;[1 1 1] trace line
                  (`/Game/GameFPS/Widgets/WBP_PlayerUI.UpdateWeapon` (`self.WBP_PlayerUI`) _output_get)
                  (bind _outhit (`KismetSystemLibrary.LineTraceSingle` _returnvalue (+ _returnvalue (* (`SceneComponent.GetForwardVector` _camera) (`self.ShotRange`))) "TraceTypeQuery1" false (`|MakeArray` _bp_fps_character :!type "Actor Object Reference") "ForDuration"))
                  (bind (_bblockinghit _binitialoverlap _time _distance _location _impactpoint _normal _impactnormal _physmat _hitactor) (`GameplayStatics.BreakHitResult` _outhit))
                  ;[1 1 1] continua;ao do tiro
                  (if (`KismetSystemLibrary.DoesImplementInterface` _hitactor "/Game/GameFPS/Interfaces/BPI_Enemy.BPI_Enemy_C")
                    (message `/Game/GameFPS/Interfaces/BPI_Enemy.Hit` _hitactor (`/Game/GameFPS/core/Weapons/BP_Weapon.BaseDamage` (`self.BP_Weapon`)) _impactpoint)
                    (else
                      (bind _returnvalue_2 (`GameplayStatics.ApplyDamage` _hitactor (`/Game/GameFPS/core/Weapons/BP_Weapon.BaseDamage` (`self.BP_Weapon`))))
                      (`KismetSystemLibrary.PrintString` (`KismetStringLibrary.Conv_DoubleToString` _returnvalue_2)))))
                (:`OnCompleted`
                  (set `self.IsShooting` false))))))
        (:`else`))))
  (:`Ongoing`
    (if ActionValue
      (goto _label_2)
      (else
        (set `self.IsShooting` false)))))

(event `Key|F`
  (params (Key :type "Key Structure"))
  ;[0.6487 1 0.6273] Shot Manage
)

(event `EnhancedInput|/Game/GameFPS/Inputs/IA_Reload`
  (params (ActionValue :type Boolean) (ElapsedSeconds :type "Float (double-precision)") (TriggeredSeconds :type "Float (double-precision)") (InputAction :type "InputAction Object Reference" :default "/Game/GameFPS/Inputs/IA_Reload.IA_Reload"))
  (bind _bp_weapon (`self.BP_Weapon`))
  (bind _bp_weapon_2 (`self.BP_Weapon`))
  (bind ((`Name_11_56F88F3E450DAD7C284EAA808B049652` _name) (`MagSize_16_1C183FC04F68D2A27ACCC78AE0FCC2AE` _magsize) (`CurrentAmmo_13_4629CE37452ED34A30F90ABB1991FB87` _currentammo) (`TotalAmmo_18_BF88026740A141C2F90C73A604D54422` _totalammo) (`Category_35_C733F46047E14625B2C480A9592D084B` _category)) (break `/Game/GameFPS/Structures/S_WeaponBase` (`self.EquippedWeapon`)))
  ;[0.02083 0.02083 0.02083] Reload (manual 'R')
  (:`Started`
    (if (`self.IsReloading`)
      _
      (elif (or (<= _totalammo 0) (`self.IsShooting`) (== _magsize _currentammo))
        (`KismetSystemLibrary.PrintString` "Nao fazer nada")
        (else
          (`|PlayMontage` (`/Game/GameFPS/core/BP_FPS_Character.CharacterArms` (`self.BP FPS Character`)) "/Game/GameFPS/art/assaultRifle/animations/Montage_FP_Reload.Montage_FP_Reload" 1.0 0.0 _name
            (:`then`
              (set `self.IsReloading` true)
              (set `self.CanShoot` false))
            (:`OnCompleted`
              (set `self.IsReloading` false :!label _label_3)
              (set `self.CanShoot` true))
            (:`OnBlendOut`
              (bind _updatedweaponstats (message `/Game/GameFPS/Interfaces/BPI_Weapon.Reload` (`self.BP_Weapon`) (`self.EquippedWeapon`)))
              (bind _output_get (set `self.EquippedWeapon` _updatedweaponstats))
              (`/Game/GameFPS/Widgets/WBP_PlayerUI.UpdateWeapon` (`self.WBP_PlayerUI`) _output_get))
            (:`OnInterrupted`
              (`KismetSystemLibrary.PrintString` "interruptedReload")
              (`SceneComponent.K2_DetachFromComponent` (`/Game/GameFPS/core/Weapons/BP_Weapon.SM_Mag` (`self.BP_Weapon`)) "KeepRelative" "KeepRelative" "KeepRelative" true)
              (`SceneComponent.K2_AttachToComponent` (`/Game/GameFPS/core/Weapons/BP_Weapon.SM_Mag` _bp_weapon) (`/Game/GameFPS/core/Weapons/BP_Weapon.SK_Gun` _bp_weapon) (`/Game/GameFPS/core/Weapons/BP_Weapon.MagSocketName` _bp_weapon) "KeepRelative" "KeepRelative" "KeepRelative" true)
              (`KismetSystemLibrary.Delay` 1.0)
              (goto _label_3))
            (:`OnNotifyBegin`
              (`SceneComponent.K2_DetachFromComponent` (`/Game/GameFPS/core/Weapons/BP_Weapon.SM_Mag` (`self.BP_Weapon`)) "KeepRelative" "KeepRelative" "KeepRelative" true)
              (switch `/Game/GameFPS/Enumerators/E_WeaponCategory` _category
                (:`NewEnumerator0`
                  (`SceneComponent.K2_AttachToComponent` (`/Game/GameFPS/core/Weapons/BP_Weapon.SM_Mag` (`self.BP_Weapon`)) (`/Game/GameFPS/core/BP_FPS_Character.CharacterArms` (`self.BP FPS Character`)) "Rifle0_magSocket" "KeepRelative" "KeepRelative" "KeepRelative" true))
                (:`NewEnumerator1`
                  (`SceneComponent.K2_AttachToComponent` (`/Game/GameFPS/core/Weapons/BP_Weapon.SM_Mag` (`self.BP_Weapon`)) (`/Game/GameFPS/core/BP_FPS_Character.CharacterArms` (`self.BP FPS Character`)) "Rifle1_magSocket" "KeepRelative" "KeepRelative" "KeepRelative" true))))
            (:`OnNotifyEnd`
              (`SceneComponent.K2_DetachFromComponent` (`/Game/GameFPS/core/Weapons/BP_Weapon.SM_Mag` (`self.BP_Weapon`)) "KeepRelative" "KeepRelative" "KeepRelative" true)
              (`SceneComponent.K2_AttachToComponent` (`/Game/GameFPS/core/Weapons/BP_Weapon.SM_Mag` _bp_weapon_2) (`/Game/GameFPS/core/Weapons/BP_Weapon.SK_Gun` _bp_weapon_2) (`/Game/GameFPS/core/Weapons/BP_Weapon.MagSocketName` _bp_weapon_2) "KeepRelative" "KeepRelative" "KeepRelative" true))))))))

(fn `UpdateEquippedWeapon`
  (params (EquippedWeapon :type "/Game/GameFPS/Structures/S_WeaponBase Structure") (BP_Weapon :type "/Game/GameFPS/core/Weapons/BP_Weapon Object Reference"))
  (set `self.BP_Weapon` BP_Weapon)
  (set `self.EquippedWeapon` EquippedWeapon)
  (`/Game/GameFPS/Widgets/WBP_PlayerUI.UpdateWeapon` (`self.WBP_PlayerUI`) (`self.EquippedWeapon`))
  (set `self.IsEquipped` true))