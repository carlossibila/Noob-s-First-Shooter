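; Player inventory component for the FPS character, managing a primary and a secondary weapon slot plus access to the gun store.
; BeginPlay fills the store widget from DT_Weapons and caches level-placed BP_Weapon actors, whose classes are spawned by index when adding to empty slots.
; The store opens only when CanBuy is set.
; Equip inputs, blocked while shooting or reloading, attach the slot's weapon to the arms and update BPCEquippedWeapon.
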(event `self.ReceiveBeginPlay`
  (`|ExecutionSequence`
    (:`then_0`
      (`KismetSystemLibrary.PrintString` "inicializada" true true (struct :`G` 0.66 :`B` 1.0 :`A` 1.0) 60.0)
      (bind _asbp_fps_character (cast `/Game/GameFPS/core/BP_FPS_Character` (`GameplayStatics.GetPlayerCharacter` 0)))
      (bind _output_get (set `self.BP FPS Character` _asbp_fps_character))
      (set `self.BPC Equipped Weapon` (`/Game/GameFPS/core/BP_FPS_Character.BPC_EquippedWeapon` _output_get)))
    (:`then_1`
      (`EnhancedInputSubsystemInterface.AddMappingContext` (pcsubsystem `EnhancedInputLocalPlayerSubsystem` (`GameplayStatics.GetPlayerController` 0)) "/Game/GameFPS/Inputs/IMC_GunStore.IMC_GunStore" 0 (struct)))
    (:`then_2`
      (`KismetArrayLibrary.Array_Resize` (`self.StoreWeapons`) 2)
      (`KismetArrayLibrary.Array_Resize` (`self.PlayerInventory`) 2)
      (`KismetArrayLibrary.Array_Resize` (`self.BP_WeaponArray`) 2))
    (:`then_3`
      ;[1 1 1] add items to store array
      (bind _outrownames (`DataTableFunctionLibrary.GetDataTableRowNames` "/Game/GameFPS/DataTables/DT_Weapons.DT_Weapons"))
      (for (_array_element _array_index) _outrownames
        (bind _returnvalue (`|GetDataTableRow` "/Game/GameFPS/DataTables/DT_Weapons.DT_Weapons" _array_element)
          (:`then`
            (`KismetArrayLibrary.Array_Set` (`self.StoreWeapons`) _array_index _returnvalue)))))
    (:`then_4`
      (bind _returnvalue_2 (`|CreateWidget` "/Game/GameFPS/Widgets/WBP_GunStore.WBP_GunStore_C" null (`self.StoreWeapons`)))
      (set `self.WBP_GunStore` _returnvalue_2))
    (:`then_5`
      ;[1 1 1] get all weapon classes
      (bind _outactors (`GameplayStatics.GetAllActorsOfClass` "/Game/GameFPS/core/Weapons/BP_Weapon.BP_Weapon_C"))
      (`KismetArrayLibrary.Array_Remove` _outactors)
      (set `self.BP_WeaponArray` _outactors))))

(event `EnhancedInput|/Game/GameFPS/Inputs/IA_OpenStore`
  (params (ActionValue :type Boolean) (ElapsedSeconds :type "Float (double-precision)") (TriggeredSeconds :type "Float (double-precision)") (InputAction :type "InputAction Object Reference" :default "/Game/GameFPS/Inputs/IA_OpenStore.IA_OpenStore"))
  (bind _returnvalue (`GameplayStatics.GetPlayerController` 0))
  (bind _wbp_gunstore (`self.WBP_GunStore`))
  ;[1 1 1] openStore  -  checks store limits
  (:`Triggered`
    (if (`self.CanBuy`)
      (`Actor.DisableInput` (`self.BP FPS Character`) _returnvalue)
      (`WidgetBlueprintLibrary.SetInputMode_UIOnlyEx` _returnvalue null)
      (set `PlayerController.bShowMouseCursor` true _returnvalue)
      (`UserWidget.AddToViewport` _wbp_gunstore 0)
      (`Widget.SetFocus` _wbp_gunstore)
      (else
        (`KismetSystemLibrary.PrintString` "Outside Store Limits")))))

(event `EnhancedInput|/Game/GameFPS/Inputs/IA_Equip1`
  (params (ActionValue :type Boolean) (ElapsedSeconds :type "Float (double-precision)") (TriggeredSeconds :type "Float (double-precision)") (InputAction :type "InputAction Object Reference" :default "/Game/GameFPS/Inputs/IA_Equip1.IA_Equip1"))
  (bind _bpc_equipped_weapon (`self.BPC Equipped Weapon`))
  ;[0.845 1 0.1633] review that condition for cancel reload and change weapon
  (:`Started`
    (if (not (or (`/Game/GameFPS/Components/BPC_EquippedWeapon.IsShooting` _bpc_equipped_weapon) (`/Game/GameFPS/Components/BPC_EquippedWeapon.IsReloading` _bpc_equipped_weapon)))
      (bind _output_get (set `self.InventoryIndex` 0))
      (`/Engine/EditorBlueprintResources/StandardMacros.IsValid` (`|GetArrayItem` (`self.PlayerInventory`) _output_get)
        (:`Is Valid`
          (bind _equippedweapon (`self.Equip Weapon` _output_get))
          (`/Game/GameFPS/Components/BPC_EquippedWeapon.UpdateEquippedWeapon` (`self.BPC Equipped Weapon`) _equippedweapon (`self.EquippedWeapon`)))
        (:`Is Not Valid`
          (`KismetSystemLibrary.PrintString` "nada nesse slot 0"))))))

(event `EnhancedInput|/Game/GameFPS/Inputs/IA_Equip2`
  (params (ActionValue :type Boolean) (ElapsedSeconds :type "Float (double-precision)") (TriggeredSeconds :type "Float (double-precision)") (InputAction :type "InputAction Object Reference" :default "/Game/GameFPS/Inputs/IA_Equip2.IA_Equip2"))
  (bind _bpc_equipped_weapon (`self.BPC Equipped Weapon`))
  ;[0.845 1 0.1633] review that condition for cancel reload and change weapon
  (:`Started`
    (if (not (or (`/Game/GameFPS/Components/BPC_EquippedWeapon.IsShooting` _bpc_equipped_weapon) (`/Game/GameFPS/Components/BPC_EquippedWeapon.IsReloading` _bpc_equipped_weapon)))
      (bind _output_get (set `self.InventoryIndex` 1))
      (`/Engine/EditorBlueprintResources/StandardMacros.IsValid` (`|GetArrayItem` (`self.PlayerInventory`) _output_get)
        (:`Is Valid`
          (bind _equippedweapon (`self.Equip Weapon` _output_get))
          (`/Game/GameFPS/Components/BPC_EquippedWeapon.UpdateEquippedWeapon` (`self.BPC Equipped Weapon`) _equippedweapon (`self.EquippedWeapon`)))
        (:`Is Not Valid`
          (`KismetSystemLibrary.PrintString` "nada nesse slot 1"))))))

(fn `Add to Player Inventory`
  (params (BoughtWeaponType :type "/Game/GameFPS/Enumerators/E_WeaponType Enum" :default "NewEnumerator0") (FetchIndex :type Integer))
  (returns (success :type Boolean))
  (set `self.FetchIndex` FetchIndex)
  (switch `/Game/GameFPS/Enumerators/E_WeaponType` BoughtWeaponType
    (:`NewEnumerator0`
      (bind _output_get (set `self.InventoryIndex` 0))
      (`/Engine/EditorBlueprintResources/StandardMacros.IsValid` (`|GetArrayItem` (`self.PlayerInventory`) _output_get)
        (:`Is Valid`
          (`KismetSystemLibrary.PrintString` "slot ocupado")
          (return false))
        (:`Is Not Valid`
          (`KismetSystemLibrary.PrintString` "slot vazio")
          (bind _returnvalue (`|SpawnActorFromClass` (`GameplayStatics.GetObjectClass` (`|GetArrayItem` (`self.BP_WeaponArray`) (`self.FetchIndex`))) (`KismetMathLibrary.MakeTransform` (0.0 0.0 -200.0)) "Undefined" "MultiplyWithRoot" null null))
          (`KismetArrayLibrary.Array_Set` (`self.PlayerInventory`) (`self.InventoryIndex`) _returnvalue)
          (return true))))
    (:`NewEnumerator1`
      (bind _output_get_2 (set `self.InventoryIndex` 1))
      (`/Engine/EditorBlueprintResources/StandardMacros.IsValid` (`|GetArrayItem` (`self.PlayerInventory`) _output_get_2)
        (:`Is Valid`
          (`KismetSystemLibrary.PrintString` "slot ocupado")
          (return false))
        (:`Is Not Valid`
          (`KismetSystemLibrary.PrintString` "slot vazio")
          (bind _returnvalue_2 (`|SpawnActorFromClass` (`GameplayStatics.GetObjectClass` (`|GetArrayItem` (`self.BP_WeaponArray`) (`self.FetchIndex`))) (`KismetMathLibrary.MakeTransform` (0.0 0.0 -200.0)) "Undefined" "MultiplyWithRoot" null null))
          (`KismetArrayLibrary.Array_Set` (`self.PlayerInventory`) (`self.InventoryIndex`) _returnvalue_2)
          (return true))))))

(fn `Equip Weapon`
  (params (Index :type Integer))
  (returns (EquippedWeapon :type "/Game/GameFPS/Structures/S_WeaponBase Structure"))
  (bind _output (`|GetArrayItem` (`self.PlayerInventory`) Index))
  ;[1 1 1] LimaDuarte
  (bind _equippedweapon (`self.EquippedWeapon`)
    (:`then`
      (`Actor.K2_DetachFromActor` _equippedweapon "KeepRelative" "KeepRelative" "KeepRelative")
      (`SceneComponent.SetVisibility` (`/Game/GameFPS/core/Weapons/BP_Weapon.SK_Gun` _equippedweapon) false false))
    (:`else`
      _))
  (`Actor.K2_AttachToComponent` _output (`/Game/GameFPS/core/BP_FPS_Character.CharacterArms` (`self.BP FPS Character`)) "ik_hand_gun" "SnapToTarget" "SnapToTarget" "SnapToTarget" true)
  (bind _output_get (set `self.EquippedWeapon` _output))
  (`SceneComponent.SetVisibility` (`/Game/GameFPS/core/Weapons/BP_Weapon.SK_Gun` _output_get) true false)
  (return (`/Game/GameFPS/core/Weapons/BP_Weapon.S_WeaponBase` _output_get)))

(fn `RemoveFromPlayerInventory`
  (params (RemoveIndex :type Integer))
  (if (`/Game/GameFPS/Components/BPC_EquippedWeapon.IsEquipped` (`self.BPC Equipped Weapon`))
    (`KismetSystemLibrary.PrintString` "DropWeapon"))
  (`KismetArrayLibrary.Array_Set` (`self.PlayerInventory`) RemoveIndex))