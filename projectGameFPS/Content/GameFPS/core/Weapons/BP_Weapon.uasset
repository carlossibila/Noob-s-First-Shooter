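; Weapon actor for the FPS player that fires bullets and manages magazine and reserve ammo through the SWeaponBase struct.
; The construction script applies the skeletal mesh and selects magazine socket and base damage by category.
; Shot decrements ammo, spawns BP_Bullet at the character's BulletSpawn and sets the Reload flag on empty, blocking further fire.
; Shot and Reload take a weapon struct and return the rebuilt state; Reload refills from reserve.
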(event `self.ReceiveBeginPlay`
  (bind _asbp_fps_character (cast `/Game/GameFPS/core/BP_FPS_Character` (`GameplayStatics.GetPlayerCharacter` 0)))
  (set `self.As BP FPS Character` _asbp_fps_character))

(fn `BulletFling`
  (switch `/Game/GameFPS/Enumerators/E_WeaponCategory` (`.Category_35_C733F46047E14625B2C480A9592D084B` (break `/Game/GameFPS/Structures/S_WeaponBase` (`self.S_WeaponBase`)))
    (:`NewEnumerator0`
      (`|SpawnActorFromClass` "/Game/GameFPS/core/Weapons/Projectile/BP_Bullet.BP_Bullet_C" (`SceneComponent.K2_GetComponentToWorld` (`/Game/GameFPS/core/BP_FPS_Character.BulletSpawn` (`self.As BP FPS Character`))) "Undefined" "MultiplyWithRoot" null null))
    (:`NewEnumerator1`
      (`|SpawnActorFromClass` "/Game/GameFPS/core/Weapons/Projectile/BP_Bullet.BP_Bullet_C" (`SceneComponent.K2_GetComponentToWorld` (`/Game/GameFPS/core/BP_FPS_Character.BulletSpawn` (`self.As BP FPS Character`))) "Undefined" "MultiplyWithRoot" null null))))

(fn `Reload`
  (params (SourceWeapon :type "/Game/GameFPS/Structures/S_WeaponBase Structure"))
  (returns (UpdatedWeaponStats :type "/Game/GameFPS/Structures/S_WeaponBase Structure"))
  (bind (_weaponid _name _sk_weapon _reload _magsize _currentammo _totalammo _killrevenue _firerate _type _category) (break `/Game/GameFPS/Structures/S_WeaponBase` SourceWeapon))
  (bind _returnvalue (- _magsize _currentammo))
  (bind _returnvalue_2 (- _totalammo _returnvalue))
  (if (or (== _magsize _currentammo) (<= _totalammo 0))
    (if (== _currentammo 0)
      (bind _output_get (set `self.S_WeaponBase` (make `/Game/GameFPS/Structures/S_WeaponBase` _weaponid _name _sk_weapon true _magsize _currentammo _totalammo _killrevenue _firerate _type _category)))
      (`GameplayStatics.PlaySoundAtLocation` "/Engine/VREditor/Sounds/UI/Invalid_Action.Invalid_Action" (`SceneComponent.K2_GetComponentLocation` (`self.SK_Gun`)) (struct) 1.0 1.0 0.0 null null null null)
      (return _output_get)
      (else
        (bind _output_get_2 (set `self.S_WeaponBase` (make `/Game/GameFPS/Structures/S_WeaponBase` _weaponid _name _sk_weapon false _magsize _currentammo _totalammo _killrevenue _firerate _type _category)))
        (return _output_get_2)))
    (elif (< _returnvalue_2 0)
      (bind _output_get_3 (set `self.S_WeaponBase` (make `/Game/GameFPS/Structures/S_WeaponBase` _weaponid _name _sk_weapon false _magsize _totalammo 0 _killrevenue _firerate _type _category)))
      (return _output_get_3)
      (else
        (bind _output_get_4 (set `self.S_WeaponBase` (make `/Game/GameFPS/Structures/S_WeaponBase` _weaponid _name _sk_weapon false _magsize (+ _returnvalue _currentammo) _returnvalue_2 _killrevenue _firerate _type _category)))
        (return _output_get_4)))))

(fn `Shot`
  (params (SourceWeapon :type "/Game/GameFPS/Structures/S_WeaponBase Structure"))
  (returns (UpdatedWeaponStats :type "/Game/GameFPS/Structures/S_WeaponBase Structure"))
  (bind (_weaponid _name _sk_weapon _reload _magsize _currentammo _totalammo _killrevenue _firerate _type _category) (break `/Game/GameFPS/Structures/S_WeaponBase` SourceWeapon))
  (bind (_weaponid_2 _name_2 _sk_weapon_2 _reload_2 _magsize_2 _currentammo_2 _totalammo_2 _killrevenue_2 _firerate_2 _type_2 _category_2) (break `/Game/GameFPS/Structures/S_WeaponBase` (`self.S_WeaponBase`)))
  (if _reload
    (return (`self.S_WeaponBase`))
    (else
      (bind _result (`/Engine/EditorBlueprintResources/StandardMacros.DecrementInt` _currentammo)
        (:`  `
          (bind _output_get (set `self.S_WeaponBase` (make `/Game/GameFPS/Structures/S_WeaponBase` _weaponid _name _sk_weapon _reload _magsize _result _totalammo _killrevenue _firerate _type _category)))
          (`self.BulletFling`)
          (if (!= (`.CurrentAmmo_13_4629CE37452ED34A30F90ABB1991FB87` (break `/Game/GameFPS/Structures/S_WeaponBase` (`self.S_WeaponBase`))) 0)
            (return _output_get)
            (else
              (bind _output_get_2 (set `self.S_WeaponBase` (make `/Game/GameFPS/Structures/S_WeaponBase` _weaponid_2 _name_2 _sk_weapon_2 true _magsize_2 _currentammo_2 _totalammo_2 _killrevenue_2 _firerate_2 _type_2 _category_2)))
              (return _output_get_2))))))))

(fn `UserConstructionScript`
  (bind ((`SK_Weapon_22_E2F5BE044449A22D68E4F58E8C3670AE` _sk_weapon) (`Category_35_C733F46047E14625B2C480A9592D084B` _category)) (break `/Game/GameFPS/Structures/S_WeaponBase` (`self.S_WeaponBase`)))
  (`SkeletalMeshComponent.SetSkeletalMeshAsset` (`self.SK_Gun`) _sk_weapon)
  (switch `/Game/GameFPS/Enumerators/E_WeaponCategory` _category
    (:`NewEnumerator0`
      (set `self.MagSocketName` "Magazine")
      (set `self.BaseDamage` 13.0))
    (:`NewEnumerator1`
      (set `self.MagSocketName` "Stanag_Mag")
      (set `self.BaseDamage` 19.0))))