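; Honey Badger weapon Blueprint, a child that relies on its parent class for all gameplay behavior.
; Its construction script runs the parent's, then sets the SMMag component to the assault rifle magazine mesh and attaches it to SKGun at the MagSocketName socket, keeping relative transforms.
; The event graph holds only disabled default event stubs.
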(fn `UserConstructionScript`
  (`parent.UserConstructionScript`)
  (`StaticMeshComponent.SetStaticMesh` (`self.SM_Mag`) "/Game/GameFPS/art/assaultRifle/meshes/SM_AssaultRifle_Magazine.SM_AssaultRifle_Magazine")
  (`SceneComponent.K2_AttachToComponent` (`self.SM_Mag`) (`self.SK_Gun`) (`self.MagSocketName`) "KeepRelative" "KeepRelative" "KeepRelative" true))