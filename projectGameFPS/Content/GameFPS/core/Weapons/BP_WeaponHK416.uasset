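; BP_WeaponHK416 is the HK416 weapon Blueprint, a child that builds on its parent's gun and magazine setup.
; After running the parent construction script, it hides the Stanag_Mag bone on the gun's skeletal mesh.
; It then assigns the empty HK416 magazine static mesh and attaches it to the gun at the magazine socket.
; Its event graph holds only disabled stubs, so it adds no runtime logic.
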(fn `UserConstructionScript`
  (`parent.UserConstructionScript`)
  (`SkinnedMeshComponent.HideBoneByName` (`self.SK_Gun`) "Stanag_Mag" "PBO_None")
  (`StaticMeshComponent.SetStaticMesh` (`self.SM_Mag`) "/Game/GameFPS/art/Assets/Guns/ProjectilesAndMags/SM_HK416_MagEmpty.SM_HK416_MagEmpty")
  (`SceneComponent.K2_AttachToComponent` (`self.SM_Mag`) (`self.SK_Gun`) (`self.MagSocketName`) "KeepRelative" "KeepRelative" "KeepRelative" true))