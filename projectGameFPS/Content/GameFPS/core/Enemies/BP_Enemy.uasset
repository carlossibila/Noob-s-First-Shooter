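; BP_Enemy is an enemy pawn that chases pawns it sees, damages them and dies when its health runs out.
; PawnSensing triggers AIMoveTo toward the seen pawn, and a successful move applies fixed damage to it.
; AnyDamage reduces EnemyTotalHealth; a lethal hit spawns a Niagara fire effect using the EvilCube's X/Y position, then destroys the actor.
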(event `self.PawnSensing.OnSeePawn`
  (params (Pawn :type "Pawn Object Reference"))
  (`KismetSystemLibrary.PrintString` "see")
  (`|AIMoveTo` self (0.0 0.0 0.0) Pawn
    (:`OnSuccess`
      (`GameplayStatics.ApplyDamage` Pawn 10.0))))

(event `self.ReceiveAnyDamage`
  (params (Damage :type "Float (single-precision)") (DamageType :type "DamageType Object Reference") (InstigatedBy :type "Controller Object Reference") (DamageCauser :type "Actor Object Reference"))
  (bind (_returnvalue_x _returnvalue_y) (`KismetMathLibrary.BreakVector` (`SceneComponent.K2_GetComponentLocation` (`self.EvilCube`))))
  (bind _returnvalue (- (`self.EnemyTotalHealth`) Damage))
  (if (<= _returnvalue 0.0)
    (`NiagaraFunctionLibrary.SpawnSystemAtLocation` "/Game/MixedVFX/Particles/Fires/NS_BigFire.NS_BigFire" (`KismetMathLibrary.MakeVector` _returnvalue_x _returnvalue_y))
    (`self.K2_DestroyActor`)
    (else
      (set `self.EnemyTotalHealth` _returnvalue))))

(fn `UserConstructionScript`)