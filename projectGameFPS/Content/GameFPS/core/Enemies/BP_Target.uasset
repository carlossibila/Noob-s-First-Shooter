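; BP_Target is a shootable barrel target that explodes when its life points run out.
; Its Hit event subtracts incoming damage from TargetLifePoints and spawns a Niagara hit effect at the impact location while it survives.
; At zero or below, it spawns a large explosion effect at the BarrelTarget component, applies radial damage around it and destroys itself.
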(event `/Game/GameFPS/Interfaces/BPI_Enemy.Hit`
  (params (DamageApply :type "Float (double-precision)") (LocationApply :type "Vector Structure"))
  ;[1 1 1] hitDamage
  (bind _output_get (set `self.TargetLifePoints` (- (`self.TargetLifePoints`) DamageApply)))
  (if (<= _output_get 0.0)
    (`NiagaraFunctionLibrary.SpawnSystemAtLocation` "/Game/MixedVFX/Particles/Explosions/NS_ExplosionGroundBig.NS_ExplosionGroundBig" (`SceneComponent.K2_GetComponentLocation` (`self.BarrelTarget`)))
    (`GameplayStatics.ApplyRadialDamage` :`BaseDamage` 50.0 :`Origin` (`SceneComponent.K2_GetComponentLocation` (`self.BarrelTarget`)) :`DamageRadius` 1000.0 :`DamageCauser` null :`InstigatedByController` null)
    (`self.K2_DestroyActor`)
    (else
      (`NiagaraFunctionLibrary.SpawnSystemAtLocation` "/Game/MixedVFX/Particles/Projectiles/Hits/NS_FireArrow_Hit.NS_FireArrow_Hit" LocationApply))))

(fn `UserConstructionScript`)